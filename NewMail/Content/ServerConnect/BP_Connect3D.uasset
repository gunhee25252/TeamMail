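; BP_Connect3D fetches textures from a server folder (URL plus Name) and applies them to its static mesh components at runtime.
; On BeginPlay, ImageDownloader requests the images, and each arrival stores the texture and creates a dynamic material on the mesh matching its request index.
; After a fixed short delay, SetMat sets each "Color" parameter, without waiting for downloads and assuming arrival order matches request index.
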(event `self.ReceiveBeginPlay`
  (bind _imagedownloader (`self.ImageDownloader`))
  (bind _returnvalue (`KismetStringLibrary.Concat_StrStr` (`self.URL`) (`self.Name`)))
  (`KismetArrayLibrary.Array_Clear` (`self.StaticMeshes`))
  (`KismetArrayLibrary.Array_Clear` (`self.DMI_Mat`))
  (`BlueprintMapLibrary.Map_Clear` (`self.LoadedTextures`))
  (set `self.StaticMeshes` (`self.K2_GetComponentsByClass` "/Script/Engine.StaticMeshComponent"))
  (add `ImageDownloaderComponent.OnTextureLoaded` _imagedownloader (delegate `LoadTexture`))
  (`ImageDownloaderComponent.DownloadImagesByUrlFolder` _imagedownloader _returnvalue _returnvalue)
  (`KismetSystemLibrary.Delay` 0.3)
  (`self.SetMat`))

(event `LoadTexture`
  (params (LoadedTexture :type "Texture2D Object Reference") (RequestIndex :type Integer))
  (`BlueprintMapLibrary.Map_Add` (`self.LoadedTextures`) RequestIndex LoadedTexture)
  (bind _returnvalue (`PrimitiveComponent.CreateDynamicMaterialInstance` (`|GetArrayItem` (`self.StaticMeshes`) RequestIndex) 0 (`|GetArrayItem` (`self.Materials`) RequestIndex) (`KismetStringLibrary.Conv_StringToName` (`KismetStringLibrary.Concat_StrStr` "MID" (`KismetStringLibrary.Conv_IntToString` RequestIndex)))))
  (`KismetArrayLibrary.Array_Add` (`self.DMI_Mat`) _returnvalue))

(event `SetMat`
  (bind _loadedtextures (`self.LoadedTextures`))
  (bind _keys (`BlueprintMapLibrary.Map_Keys` _loadedtextures))
  (for _array_element _keys
    (bind _values (`BlueprintMapLibrary.Map_Values` _loadedtextures))
    (`MaterialInstanceDynamic.SetTextureParameterValue` (`|GetArrayItem` (`self.DMI_Mat`) _array_element) "Color" (`|GetArrayItem` _values _array_element))))

(fn `UserConstructionScript`)