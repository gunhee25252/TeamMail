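; BP_Connect2D downloads an image from a server at play start and shows it as a texture on its 00 component.
; An ImageDownloader fetches the address built from URL and Name, and its loaded callback stores the texture and creates a dynamic instance of MI_00.
; SetMat runs once after a short fixed delay, independent of that callback, and sets the Color parameter only if the material instance already exists.
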(event `self.ReceiveBeginPlay`
  (bind _imagedownloader (`self.ImageDownloader`))
  (add `ImageDownloaderComponent.OnTextureLoaded` _imagedownloader (delegate `LoadTexture`))
  (`ImageDownloaderComponent.DownloadImageFromURL` _imagedownloader (`KismetStringLibrary.Concat_StrStr` (`self.URL`) (`self.Name`)) 0)
  (`KismetSystemLibrary.Delay` 0.2)
  (`self.SetMat`))

(event `LoadTexture`
  (params (LoadedTexture :type "Texture2D Object Reference") (RequestIndex :type Integer))
  (set `self.LoadedTextures` LoadedTexture)
  (bind _returnvalue (`PrimitiveComponent.CreateDynamicMaterialInstance` (`self.00`) 0 "/Game/ServerConnect/Material/MI_00.MI_00" "MID_00"))
  (set `self.DMI_Mat` _returnvalue))

(event `SetMat`
  (bind _dmi_mat (`self.DMI_Mat`))
  (`/Engine/EditorBlueprintResources/StandardMacros.IsValid` _dmi_mat
    (:`Is Valid`
      (`MaterialInstanceDynamic.SetTextureParameterValue` _dmi_mat "Color" (`self.LoadedTextures`)))))

(fn `UserConstructionScript`)