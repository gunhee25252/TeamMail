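; Function library for modular doors, supplying meshes, sizing and transforms for doors, frames, top windows and handles.
; GetDoorDetails maps AU, DIN EN and US standard sizes to six base size classes plus width and height scale factors.
; Mesh getters read per-style DataTable rows and pick the mesh for a size class, with separate glass rows where needed.
; Custom-scale helpers fit arbitrary door meshes using their bounds and yaw bucketed into 90-degree orientations.
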(fn `Add Offset Z`
  (params (InTransform :type "Transform Structure (by ref)") (Offset :type "Float (double-precision)"))
  (returns (Transform :type "Transform Structure"))
  (return (`KismetMathLibrary.MakeTransform` (`KismetMathLibrary.MakeVector` (.x (.location InTransform)) (.y (.location InTransform)) (+ Offset (.z (.location InTransform)))) (.rotation InTransform) (.scale InTransform))))

(fn `Combine Transforms`
  (params (`Transform 1` :type "Transform Structure (by ref)") (`Transform 2` :type "Transform Structure (by ref)"))
  (returns (Combined :type "Transform Structure"))
  (return (`KismetMathLibrary.MakeTransform` (+ (.location `Transform 1`) (.location `Transform 2`)) (`KismetMathLibrary.ComposeRotators` (.rotation `Transform 1`) (.rotation `Transform 2`)) (* (.scale `Transform 1`) (.scale `Transform 2`)))))

(fn `Get Custom Scale`
  (params (size :type "/Game/3dAsset/DoorsBPV2/Blueprints/Enums/Enum_DoorSizes Enum" :default "NewEnumerator12") (DoorMesh :type "StaticMesh Object Reference") (ThicknessScale :type "Float (double-precision)" :default 1.0) (Transform :type "Transform Structure"))
  (returns (Scale :type "Vector Structure") (Offset :type "Vector Structure"))
  (bind (_origin _boxextent) (`KismetMathLibrary.BreakBoxSphereBounds` (`StaticMesh.GetBounds` DoorMesh)))
  (bind _yaw (.yaw (.rotation Transform)))
  (bind _x (.x _origin))
  (bind _y (.y _origin))
  (bind _x_2 (.x _boxextent))
  (bind _y_2 (.y _boxextent))
  (bind _returnvalue (select `/Game/3dAsset/DoorsBPV2/Blueprints/Enums/Enum_SizeType` (`.Size_31_B8433DE84B64E774499717A1BF6F598E` (break `/Game/3dAsset/DoorsBPV2/Blueprints/Structs/BPS_DoorSizes` (`self.Get Door Details` size))) :`NewEnumerator0` (36.0 4.0 102.0) :`NewEnumerator1` (41.0 4.0 102.0) :`NewEnumerator2` (46.0 4.0 102.0) :`NewEnumerator3` (36.0 4.0 117.0) :`NewEnumerator4` (41.0 4.0 117.0) :`NewEnumerator5` (46.0 4.0 117.0) :!type "Vector Structure"))
  (bind _returnvalue_2 (* _x ThicknessScale))
  (bind _returnvalue_3 (* _y ThicknessScale))
  (bind _returnvalue_4 (/ (.z _returnvalue) (.z _boxextent)))
  (bind _returnvalue_5 (/ (.x _returnvalue) (.x _boxextent)))
  (bind _returnvalue_6 (/ (.x _returnvalue) (.y _boxextent)))
  (bind _returnvalue_7 (`KismetMathLibrary.MakeVector` ThicknessScale _returnvalue_6 _returnvalue_4))
  (bind _returnvalue_8 (`KismetMathLibrary.MakeVector` _returnvalue_5 ThicknessScale (/ (.z _returnvalue) (.z _boxextent))))
  (bind _returnvalue_9 (select `bool` (< _yaw 5.0) :`false` (select `bool` (< _yaw 95.0) :`false` (select `bool` (< _yaw 185.0) :`false` "NewEnumerator3" :`true` "NewEnumerator2" :!type "/Game/3dAsset/DoorsBPV2/Blueprints/Enums/Enum_Rotation Enum") :`true` "NewEnumerator1") :`true` "NewEnumerator0"))
  (bind _returnvalue_10 (* (select `/Game/3dAsset/DoorsBPV2/Blueprints/Enums/Enum_Rotation` _returnvalue_9 :`NewEnumerator0` (- _y _y_2) :`NewEnumerator1` (- _x _x_2) :`NewEnumerator2` (+ _y _y_2) :`NewEnumerator3` (+ _x _x_2)) (select `/Game/3dAsset/DoorsBPV2/Blueprints/Enums/Enum_Rotation` _returnvalue_9 :`NewEnumerator0` _returnvalue_6 :`NewEnumerator1` _returnvalue_5 :`NewEnumerator2` _returnvalue_6 :`NewEnumerator3` _returnvalue_5) -1.0))
  (`|ExecutionSequence`
    (:`then_1`
      (`/Engine/EditorBlueprintResources/StandardMacros.IsValid` DoorMesh
        (:`Is Valid`
          (return (select `/Game/3dAsset/DoorsBPV2/Blueprints/Enums/Enum_Rotation` _returnvalue_9 :`NewEnumerator0` _returnvalue_7 :`NewEnumerator1` _returnvalue_8 :`NewEnumerator2` _returnvalue_7 :`NewEnumerator3` _returnvalue_8) (`KismetMathLibrary.MakeVector` (select `/Game/3dAsset/DoorsBPV2/Blueprints/Enums/Enum_Rotation` _returnvalue_9 :`NewEnumerator0` (- -2.0 _returnvalue_2) :`NewEnumerator1` _returnvalue_10 :`NewEnumerator2` (- 2.0 _returnvalue_2) :`NewEnumerator3` _returnvalue_10) (select `/Game/3dAsset/DoorsBPV2/Blueprints/Enums/Enum_Rotation` _returnvalue_9 :`NewEnumerator0` _returnvalue_10 :`NewEnumerator1` (- 2.0 _returnvalue_3) :`NewEnumerator2` _returnvalue_10 :`NewEnumerator3` (- -2.0 _returnvalue_3)) (* _returnvalue_4 (- (.z _boxextent) (.z _origin))))))))))

(fn `Get Door Details`
  (params (Size :type "/Game/3dAsset/DoorsBPV2/Blueprints/Enums/Enum_DoorSizes Enum" :default "NewEnumerator12"))
  (returns (DoorValues :type "/Game/3dAsset/DoorsBPV2/Blueprints/Structs/BPS_DoorSizes Structure"))
  (locals (`Door Size Structure` :type "Array of /Game/3dAsset/DoorsBPV2/Blueprints/Structs/BPS_DoorSizes Structure"))
  (bind _returnvalue (select `/Game/3dAsset/DoorsBPV2/Blueprints/Enums/Enum_DoorSizes` Size :`NewEnumerator12` 2040.0 :`NewEnumerator2` 2340.0 :`NewEnumerator9` 2040.0 :`NewEnumerator13` 2340.0 :`NewEnumerator15` 2040.0 :`NewEnumerator14` 2340.0 :`NewEnumerator0` 1972.0 :`NewEnumerator16` 2097.0 :`NewEnumerator28` 2347.0 :`NewEnumerator17` 1972.0 :`NewEnumerator18` 2097.0 :`NewEnumerator29` 2347.0 :`NewEnumerator19` 1972.0 :`NewEnumerator20` 2097.0 :`NewEnumerator30` 2347.0 :`NewEnumerator1` 2032.0 :`NewEnumerator6` 2134.0 :`NewEnumerator7` 2438.0 :`NewEnumerator11` 2032.0 :`NewEnumerator8` 2134.0 :`NewEnumerator10` 2438.0 :`NewEnumerator21` 2032.0 :`NewEnumerator22` 2134.0 :`NewEnumerator23` 2438.0 :`NewEnumerator24` 2040.0))
  (bind _returnvalue_2 (select `/Game/3dAsset/DoorsBPV2/Blueprints/Enums/Enum_DoorSizes` Size :`NewEnumerator12` "NewEnumerator0" :`NewEnumerator2` "NewEnumerator3" :`NewEnumerator9` "NewEnumerator1" :`NewEnumerator13` "NewEnumerator4" :`NewEnumerator15` "NewEnumerator2" :`NewEnumerator14` "NewEnumerator5" :`NewEnumerator0` "NewEnumerator0" :`NewEnumerator16` "NewEnumerator0" :`NewEnumerator28` "NewEnumerator3" :`NewEnumerator17` "NewEnumerator1" :`NewEnumerator18` "NewEnumerator1" :`NewEnumerator29` "NewEnumerator4" :`NewEnumerator19` "NewEnumerator2" :`NewEnumerator20` "NewEnumerator2" :`NewEnumerator30` "NewEnumerator5" :`NewEnumerator1` "NewEnumerator0" :`NewEnumerator6` "NewEnumerator0" :`NewEnumerator7` "NewEnumerator3" :`NewEnumerator11` "NewEnumerator1" :`NewEnumerator8` "NewEnumerator1" :`NewEnumerator10` "NewEnumerator4" :`NewEnumerator21` "NewEnumerator2" :`NewEnumerator22` "NewEnumerator2" :`NewEnumerator23` "NewEnumerator5" :`NewEnumerator24` "NewEnumerator1" :!type "/Game/3dAsset/DoorsBPV2/Blueprints/Enums/Enum_SizeType Enum"))
  (bind _returnvalue_3 (select `/Game/3dAsset/DoorsBPV2/Blueprints/Enums/Enum_DoorSizes` Size :`NewEnumerator12` 720.0 :`NewEnumerator2` 720.0 :`NewEnumerator9` 820.0 :`NewEnumerator13` 820.0 :`NewEnumerator15` 920.0 :`NewEnumerator14` 920.0 :`NewEnumerator0` 709.0 :`NewEnumerator16` 709.0 :`NewEnumerator28` 709.0 :`NewEnumerator17` 834.0 :`NewEnumerator18` 834.0 :`NewEnumerator29` 834.0 :`NewEnumerator19` 959.0 :`NewEnumerator20` 959.0 :`NewEnumerator30` 959.0 :`NewEnumerator1` 711.0 :`NewEnumerator6` 711.0 :`NewEnumerator7` 711.0 :`NewEnumerator11` 813.0 :`NewEnumerator8` 813.0 :`NewEnumerator10` 813.0 :`NewEnumerator21` 914.0 :`NewEnumerator22` 914.0 :`NewEnumerator23` 914.0 :`NewEnumerator24` 1.0))
  (bind _returnvalue_4 (/ _returnvalue (select `/Game/3dAsset/DoorsBPV2/Blueprints/Enums/Enum_SizeType` _returnvalue_2 :`NewEnumerator0` 2040.0 :`NewEnumerator1` 2040.0 :`NewEnumerator2` 2040.0 :`NewEnumerator3` 2340.0 :`NewEnumerator4` 2340.0 :`NewEnumerator5` 2340.0)))
  (bind _returnvalue_5 (/ _returnvalue_3 (select `/Game/3dAsset/DoorsBPV2/Blueprints/Enums/Enum_SizeType` _returnvalue_2 :`NewEnumerator0` 720.0 :`NewEnumerator1` 820.0 :`NewEnumerator2` 920.0 :`NewEnumerator3` 720.0 :`NewEnumerator4` 820.0 :`NewEnumerator5` 920.0)))
  (return (make `/Game/3dAsset/DoorsBPV2/Blueprints/Structs/BPS_DoorSizes` _returnvalue_2 (`KismetTextLibrary.Conv_TextToString` (`|FormatText` "Type {type}: {width} x {height} mm ({h} x {w})" (select `/Game/3dAsset/DoorsBPV2/Blueprints/Enums/Enum_SizeType` _returnvalue_2 :`NewEnumerator0` "S" :`NewEnumerator1` "M" :`NewEnumerator2` "L" :`NewEnumerator3` "SH" :`NewEnumerator4` "MH" :`NewEnumerator5` "LH" :!type "Text") _returnvalue_3 _returnvalue _returnvalue_5 _returnvalue_4)) _returnvalue_5 _returnvalue_4)))

(fn `Get Door Meshes`
  (params (Size :type "/Game/3dAsset/DoorsBPV2/Blueprints/Enums/Enum_SizeType Enum" :default "NewEnumerator0") (Style :type "/Game/3dAsset/DoorsBPV2/Blueprints/Enums/Enum_DoorType Enum" :default "NewEnumerator0"))
  (returns (Door :type "StaticMesh Object Reference") (Glass :type "StaticMesh Object Reference") (`Glass Mesh` :type Boolean))
  (bind _returnvalue (select `/Game/3dAsset/DoorsBPV2/Blueprints/Enums/Enum_DoorType` Style :`NewEnumerator0` "/Game/3dAsset/DoorsBPV2/Blueprints/Data/DT_TypeA.DT_TypeA" :`NewEnumerator7` "/Game/3dAsset/DoorsBPV2/Blueprints/Data/DT_TypeD.DT_TypeD" :`NewEnumerator1` "/Game/3dAsset/DoorsBPV2/Blueprints/Data/DT_TypeB.DT_TypeB" :`NewEnumerator2` "/Game/3dAsset/DoorsBPV2/Blueprints/Data/DT_TypeC.DT_TypeC" :`NewEnumerator4` "/Game/3dAsset/DoorsBPV2/Blueprints/Data/DT_TypeE.DT_TypeE" :`NewEnumerator5` "/Game/3dAsset/DoorsBPV2/Blueprints/Data/DT_Doors01.DT_Doors01" :`NewEnumerator6` "/Game/3dAsset/DoorsBPV2/Blueprints/Data/DT_Doors01.DT_Doors01" :`NewEnumerator9` "/Game/3dAsset/DoorsBPV2/Blueprints/Data/DT_Doors01.DT_Doors01" :!type "DataTable Object Reference"))
  (bind _returnvalue_2 (select `/Game/3dAsset/DoorsBPV2/Blueprints/Enums/Enum_DoorType` Style :`NewEnumerator0` "Door" :`NewEnumerator7` "Door" :`NewEnumerator1` "Door" :`NewEnumerator2` "Door" :`NewEnumerator4` "Door" :`NewEnumerator5` "04" :`NewEnumerator6` "05" :`NewEnumerator9` "Glass01" :!type "Name"))
  (switch `/Game/3dAsset/DoorsBPV2/Blueprints/Enums/Enum_DoorType` Style ; Door Type
    (:`NewEnumerator0`
      _)
    (:`NewEnumerator7`
      _)
    (:`NewEnumerator1`
      _)
    (:`NewEnumerator2`
      _)
    (:`NewEnumerator4`
      _)
    (:`NewEnumerator5`
      ;[0.5833 0.5833 0.5833 0.5] Type 01-02-03...
      (bind _returnvalue_3 (`|GetDataTableRow` _returnvalue _returnvalue_2 :!label _label)
        (:`then`
          (bind _returnvalue_4 (`|GetDataTableRow` _returnvalue (`KismetStringLibrary.Conv_StringToName` (`KismetStringLibrary.Concat_StrStr` (`KismetStringLibrary.Conv_NameToString` _returnvalue_2) "_g")))
            (:`then`
              (return (`self.Get Mesh By Size` _returnvalue_3 Size) (`self.Get Mesh By Size` _returnvalue_4 Size) true))))))
    (:`NewEnumerator6`
      (goto _label))
    (:`NewEnumerator9`
      _))
  ;[0.5833 0.5833 0.5833 0.5] Type A-B-C...
  (bind _returnvalue_5 (`|GetDataTableRow` _returnvalue _returnvalue_2)
    (:`then`
      (return (`self.Get Mesh By Size` _returnvalue_5 Size) null false))))

(fn `Get Door or Custom Meshes`
  (params (Size :type "/Game/3dAsset/DoorsBPV2/Blueprints/Enums/Enum_SizeType Enum" :default "NewEnumerator0") (Type :type "/Game/3dAsset/DoorsBPV2/Blueprints/Enums/Enum_DoorType Enum" :default "NewEnumerator8") (`Custom Door` :type "StaticMesh Object Reference") (`Custom Glass` :type "StaticMesh Object Reference"))
  (returns (Door :type "StaticMesh Object Reference") (Glass :type "StaticMesh Object Reference"))
  (bind (_door _glass) (`self.Get Door Meshes` Size Type))
  (if (`|EnumInequality` Type "NewEnumerator8")
    (return `Custom Door` `Custom Glass`)
    (else
      (return _door _glass))))

(fn `Get Door Size Offsets`
  (params (Size :type "/Game/3dAsset/DoorsBPV2/Blueprints/Enums/Enum_DoorSizes Enum" :default "NewEnumerator12") (`Handle Horizontal Offset` :type "Float (double-precision)"))
  (returns (DoorOffset :type "Float (double-precision)") (HandleOffset :type "Float (double-precision)") (TopHeightOffset :type "Float (double-precision)") (`Shutter Offset` :type "Float (double-precision)"))
  (bind _size (break `/Game/3dAsset/DoorsBPV2/Blueprints/Structs/BPS_DoorSizes` (`self.Get Door Details` Size)))
  (return (select `/Game/3dAsset/DoorsBPV2/Blueprints/Enums/Enum_SizeType` _size :`NewEnumerator0` 5.0 :`NewEnumerator2` -5.0 :`NewEnumerator3` 5.0 :`NewEnumerator5` -5.0) (- (select `/Game/3dAsset/DoorsBPV2/Blueprints/Enums/Enum_SizeType` _size :`NewEnumerator0` 72.0 :`NewEnumerator1` 82.0 :`NewEnumerator2` 92.0 :`NewEnumerator3` 72.0 :`NewEnumerator4` 82.0 :`NewEnumerator5` 92.0) `Handle Horizontal Offset`) (select `/Game/3dAsset/DoorsBPV2/Blueprints/Enums/Enum_SizeType` _size :`NewEnumerator3` 30.0 :`NewEnumerator4` 30.0 :`NewEnumerator5` 30.0) (- `Handle Horizontal Offset` 6.0)))

(fn `Get Frame Mesh`
  (params (Type :type "/Game/3dAsset/DoorsBPV2/Blueprints/Enums/Enum_FrameType Enum" :default "NewEnumerator0") (Size :type "/Game/3dAsset/DoorsBPV2/Blueprints/Enums/Enum_SizeType Enum" :default "NewEnumerator0") (isDouble :type Boolean))
  (returns (`Frame Mesh` :type "StaticMesh Object Reference") (`Door Pos Y Offset` :type "Float (double-precision)"))
  (return (`self.Get Frame Meshes` Type Size (select `bool` isDouble :`false` "Frame" :`true` "Frame2" :!type "Name")) (select `/Game/3dAsset/DoorsBPV2/Blueprints/Enums/Enum_FrameType` Type :`NewEnumerator1` -1.0 :`NewEnumerator4` -1.0)))

(fn `Get Frame Meshes`
  (params (Type :type "/Game/3dAsset/DoorsBPV2/Blueprints/Enums/Enum_FrameType Enum" :default "NewEnumerator5") (Size :type "/Game/3dAsset/DoorsBPV2/Blueprints/Enums/Enum_SizeType Enum" :default "NewEnumerator0") (RowName :type Name :default "Frame"))
  (returns (Mesh :type "StaticMesh Object Reference"))
  (bind _returnvalue (`|GetDataTableRow` (select `/Game/3dAsset/DoorsBPV2/Blueprints/Enums/Enum_FrameType` Type :`NewEnumerator0` "/Game/3dAsset/DoorsBPV2/Blueprints/Data/DT_TypeA.DT_TypeA" :`NewEnumerator1` "/Game/3dAsset/DoorsBPV2/Blueprints/Data/DT_TypeB.DT_TypeB" :`NewEnumerator2` "/Game/3dAsset/DoorsBPV2/Blueprints/Data/DT_TypeC.DT_TypeC" :`NewEnumerator4` "/Game/3dAsset/DoorsBPV2/Blueprints/Data/DT_TypeD.DT_TypeD" :!type "DataTable Object Reference") RowName)
    (:`then`
      (return (`self.Get Mesh By Size` _returnvalue Size)))))

(fn `Get Frame Transform`
  (params (BPS_DoorSizes :type "/Game/3dAsset/DoorsBPV2/Blueprints/Structs/BPS_DoorSizes Structure (by ref)") (Flipped :type Boolean) (`Thickness Scale` :type "Float (double-precision)" :default 1.0))
  (returns (`Universal Scale` :type "Vector Structure") (Transform :type "Transform Structure"))
  (bind (_size _note _scalewidth _scaleheight) (break `/Game/3dAsset/DoorsBPV2/Blueprints/Structs/BPS_DoorSizes` BPS_DoorSizes))
  (bind _returnvalue (`KismetMathLibrary.MakeVector` `Thickness Scale` (select `bool` Flipped :`false` (* -1.0 _scalewidth) :`true` _scalewidth) _scaleheight))
  (return _returnvalue (`KismetMathLibrary.MakeTransform` (0.0 0.0 0.0) (struct) _returnvalue)))

(fn `Get Handle Unscale Height`
  (params (Size :type "/Game/3dAsset/DoorsBPV2/Blueprints/Enums/Enum_DoorSizes Enum" :default "NewEnumerator12") (`Handle Height ` :type "Float (double-precision)") (`Lock Plate Offset` :type "Float (double-precision)"))
  (returns (`Scaled Height` :type "Float (double-precision)") (`Scaled Lock Offset` :type "Float (double-precision)"))
  (bind (_size _note _scalewidth _scaleheight) (break `/Game/3dAsset/DoorsBPV2/Blueprints/Structs/BPS_DoorSizes` (`self.Get Door Details` Size)))
  (return (/ `Handle Height ` _scaleheight) (/ `Lock Plate Offset` _scaleheight)))

(fn `Get Mesh By Size`
  (params (BPS_MeshBySize :type "/Game/3dAsset/DoorsBPV2/Blueprints/Structs/BPS_MeshBySize Structure (by ref)") (Size :type "/Game/3dAsset/DoorsBPV2/Blueprints/Enums/Enum_SizeType Enum" :default "NewEnumerator0"))
  (returns (Mesh :type "StaticMesh Object Reference"))
  (bind (_meshs _meshm _meshl _meshsh _meshmh _meshlh) (break `/Game/3dAsset/DoorsBPV2/Blueprints/Structs/BPS_MeshBySize` BPS_MeshBySize))
  (return (select `/Game/3dAsset/DoorsBPV2/Blueprints/Enums/Enum_SizeType` Size :`NewEnumerator0` _meshs :`NewEnumerator1` _meshm :`NewEnumerator2` _meshl :`NewEnumerator3` _meshsh :`NewEnumerator4` _meshmh :`NewEnumerator5` _meshlh)))

(fn `Get SFrame Mesh`
  (params (Type :type "/Game/3dAsset/DoorsBPV2/Blueprints/Enums/Enum_FrameType Enum" :default "NewEnumerator0") (Size :type "/Game/3dAsset/DoorsBPV2/Blueprints/Enums/Enum_SizeType Enum" :default "NewEnumerator0") (isDouble :type Boolean))
  (returns (`SD Frame Mesh` :type "StaticMesh Object Reference"))
  (return (`self.Get Frame Meshes` Type Size (select `bool` isDouble :`false` "SFrame" :`true` "SFrame2" :!type "Name"))))

(fn `Get Text Transform`
  (params (Location :type "Vector Structure") (Orientation :type Boolean))
  (returns (Transform :type "Transform Structure"))
  (return (`KismetMathLibrary.MakeTransform` Location (select `bool` Orientation :`true` (struct :`Yaw` 180.0) :!type "Rotator Structure"))))

(fn `Get Top Frame Mesh`
  (params (Type :type "/Game/3dAsset/DoorsBPV2/Blueprints/Enums/Enum_FrameType Enum" :default "NewEnumerator0") (Size :type "/Game/3dAsset/DoorsBPV2/Blueprints/Enums/Enum_SizeType Enum" :default "NewEnumerator0"))
  (returns (`Top Frame` :type "StaticMesh Object Reference") (`Top Frame Glass` :type "StaticMesh Object Reference"))
  (return (`self.Get Frame Meshes` "NewEnumerator0" Size "Top") (`self.Get Frame Meshes` "NewEnumerator0" Size "TopGlass")) ; Only Type A has a frame top atm
)

(fn `Get Top Transform`
  (params (`Top Pos` :type "Float (double-precision)") (`Window Z Offset` :type "Float (double-precision)") (`Window Z Scale` :type "Float (double-precision)") (`Size Type` :type "/Game/3dAsset/DoorsBPV2/Blueprints/Enums/Enum_SizeType Enum" :default "NewEnumerator1") (`Double Doors` :type Boolean) (`Door 2` :type Boolean))
  (returns (Transform :type "Transform Structure"))
  (bind _returnvalue (/ 79.0 86.0))
  (bind _returnvalue_2 (/ 89.0 96.0))
  (bind _returnvalue_3 (/ 99.0 106.0))
  (return (`KismetMathLibrary.MakeTransform` (`KismetMathLibrary.MakeVector` 0.0 (select `bool` `Double Doors` :`true` (select `bool` `Door 2` :`false` -3.5 :`true` (select `/Game/3dAsset/DoorsBPV2/Blueprints/Enums/Enum_SizeType` `Size Type` :`NewEnumerator0` 75.8 :`NewEnumerator1` 85.8 :`NewEnumerator2` 95.8 :`NewEnumerator3` 75.75 :`NewEnumerator4` 85.75 :`NewEnumerator5` 95.75))) (+ `Top Pos` `Window Z Offset` 212.2)) (struct) (`KismetMathLibrary.MakeVector` 1.0 (select `bool` `Double Doors` :`false` 1.0 :`true` (select `/Game/3dAsset/DoorsBPV2/Blueprints/Enums/Enum_SizeType` `Size Type` :`NewEnumerator0` _returnvalue :`NewEnumerator1` _returnvalue_2 :`NewEnumerator2` _returnvalue_3 :`NewEnumerator3` _returnvalue :`NewEnumerator4` _returnvalue_2 :`NewEnumerator5` _returnvalue_3)) `Window Z Scale`))))

(fn `GetCustomOffset`
  (params (DoorMesh :type "StaticMesh Object Reference") (`Rotation Z` :type "/Game/3dAsset/DoorsBPV2/Blueprints/Enums/Enum_Rotation Enum" :default "NewEnumerator0") (Scale :type "Vector Structure"))
  (returns (Offset :type "Vector Structure"))
  (bind _x (.x Scale))
  (bind _y (.y Scale))
  (bind (_origin _boxextent) (`KismetMathLibrary.BreakBoxSphereBounds` (`StaticMesh.GetBounds` DoorMesh)))
  (bind _x_2 (.x _origin))
  (bind _y_2 (.y _origin))
  (bind _x_3 (.x _boxextent))
  (bind _y_3 (.y _boxextent))
  (bind _returnvalue (* _x_2 _x))
  (bind _returnvalue_2 (* _y_2 _y))
  (bind _returnvalue_3 (* (select `/Game/3dAsset/DoorsBPV2/Blueprints/Enums/Enum_Rotation` `Rotation Z` :`NewEnumerator0` (- _y_2 _y_3) :`NewEnumerator1` (- _x_2 _x_3) :`NewEnumerator2` (+ _y_2 _y_3) :`NewEnumerator3` (+ _x_2 _x_3)) (select `/Game/3dAsset/DoorsBPV2/Blueprints/Enums/Enum_Rotation` `Rotation Z` :`NewEnumerator0` _y :`NewEnumerator1` _x :`NewEnumerator2` _y :`NewEnumerator3` _x) -1.0))
  (return (`KismetMathLibrary.MakeVector` (select `/Game/3dAsset/DoorsBPV2/Blueprints/Enums/Enum_Rotation` `Rotation Z` :`NewEnumerator0` (- -2.0 _returnvalue) :`NewEnumerator1` _returnvalue_3 :`NewEnumerator2` (- 2.0 _returnvalue) :`NewEnumerator3` _returnvalue_3) (select `/Game/3dAsset/DoorsBPV2/Blueprints/Enums/Enum_Rotation` `Rotation Z` :`NewEnumerator0` _returnvalue_3 :`NewEnumerator1` (- 2.0 _returnvalue_2) :`NewEnumerator2` _returnvalue_3 :`NewEnumerator3` (- -2.0 _returnvalue_2)) (* (.z Scale) (- (.z _boxextent) (.z _origin))))))

(fn `Mirror to Entry Side`
  (params (InTransform :type "Transform Structure (by ref)"))
  (returns (`Mirrored X` :type "Transform Structure"))
  (return (`KismetMathLibrary.MakeTransform` (`KismetMathLibrary.MakeVector` (+ (.x (.location InTransform)) -4.0) 0.0 (.z (.location InTransform))) (.rotation InTransform) (`KismetMathLibrary.MakeVector` (* (.x (.scale InTransform)) -1.0) (.y (.scale InTransform)) (.z (.scale InTransform))))))