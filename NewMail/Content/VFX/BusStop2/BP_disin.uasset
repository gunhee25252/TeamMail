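; Blueprint that plays a bus stop appearance effect on a skeletal mesh with an accompanying Niagara system.
; The BusStop3DIsAppear event activates Niagara and plays a timeline with its play rate scaled by TimeToComplete.
; Each update feeds the same 0-to-1 value to the mesh materials' Animation parameter and Niagara's Custom_Animation variable, keeping material and particles in sync.
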(event `BusStop3DIsAppear`
  (`ActorComponent.Activate` (`self.Niagara`) true)
  (`TimelineComponent.SetPlayRate` (`self.Timeline`) (/ 1.0 (`self.TimeToComplete`)))
  (bind (_direction _amount) (`Timeline|Timeline`)
    (:`Update`
      (bind _returnvalue (`KismetMathLibrary.Lerp` 0.0 1.0 _amount))
      (`MeshComponent.SetScalarParameterValueOnMaterials` (`self.SkeletalMesh`) "Animation" _returnvalue)
      (`NiagaraComponent.SetVariableFloat` (`self.Niagara`) "Custom_Animation" _returnvalue))))

(fn `UserConstructionScript`)