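; BP_Leaflet is a grabbable leaflet in the start room that triggers a one-time scripted moment when the player picks it up.
; The first grab sets a Hear flag, plays a start-room sound through BPSound and calls WB000 on the VRPawn.
; It then spawns a level sequence player and plays the LS_StartRoom_Seahorse sequence.
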(event `self.GrabComponent.OnGrabbed`
  (if (not (`self.Hear`))
    (set `self.Hear` true)
    (`/Game/Blueprints/StartRoom/BP_StartRoomSound.BP_StartRoomSound00` (`self.BPSound`))
    (bind _asvrpawn (cast `/Game/VRTemplate/Blueprints/VRPawn` (`GameplayStatics.GetPlayerPawn` 0)))
    (`/Game/VRTemplate/Blueprints/VRPawn.WB_000` _asvrpawn)
    (bind _outactor (`LevelSequencePlayer.CreateLevelSequencePlayer` "/Game/Sequences/StartRoom/LS_StartRoom_Seahorse.LS_StartRoom_Seahorse"))
    (`MovieSceneSequencePlayer.Play` (`LevelSequenceActor.SequencePlayer` _outactor))))

(fn `UserConstructionScript`)