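; BP_Sound is a Blueprint in the StartRoom folder that holds a timed sequence of numbered 2D audio clips.
; The sequence alternates hand-tuned Delays with PlaySound2D calls to space clips from Audio_1_54 to Audio_1_68, skipping some numbers.
; The chain is disconnected and never runs: the BP_Sound event and construction script are both empty, so the Blueprint plays nothing as it stands.
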(event `BP_Sound`)

(fn `UserConstructionScript`)