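; Start room sound Blueprint that plays a scripted sequence of audio clips, then moves the game on to the Library_00 level.
; A single custom event, BP_StartRoomSound00, runs one linear chain of non-spatial 2D sounds separated by hardcoded delays.
; The level opens after the final delay, so progression depends on fixed timing rather than on audio completion callbacks.
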(event `BP_StartRoomSound00`
  ;[1 1 1] 54
  (`KismetSystemLibrary.Delay` 5.0)
  (`GameplayStatics.PlaySound2D` "/Game/Sound/Seahorse/Audio_1_54.Audio_1_54" 1.0 1.0 0.0 null null)
  (`KismetSystemLibrary.Delay` 7.0)
  ;[1 1 1] 55
  (`GameplayStatics.PlaySound2D` "/Game/Sound/Seahorse/Audio_1_55.Audio_1_55" 1.0 1.0 0.0 null null)
  (`KismetSystemLibrary.Delay` 4.0)
  ;[1 1 1] 56
  (`GameplayStatics.PlaySound2D` "/Game/Sound/Seahorse/Audio_1_56.Audio_1_56" 1.0 1.0 0.0 null null)
  (`KismetSystemLibrary.Delay` 10.0)
  ;[1 1 1] 59
  (`GameplayStatics.PlaySound2D` "/Game/Sound/Seahorse/Audio_1_59.Audio_1_59" 1.0 1.0 0.0 null null)
  (`KismetSystemLibrary.Delay` 13.0)
  ;[1 1 1] 60
  (`GameplayStatics.PlaySound2D` "/Game/Sound/Seahorse/Audio_1_60.Audio_1_60" 1.0 1.0 0.0 null null)
  (`KismetSystemLibrary.Delay` 6.0)
  ;[1 1 1] 63
  (`GameplayStatics.PlaySound2D` "/Game/Sound/Seahorse/Audio_1_63.Audio_1_63" 1.0 1.0 0.0 null null)
  (`KismetSystemLibrary.Delay` 6.0)
  ;[1 1 1] 64
  (`GameplayStatics.PlaySound2D` "/Game/Sound/Seahorse/Audio_1_64.Audio_1_64" 1.0 1.0 0.0 null null)
  (`KismetSystemLibrary.Delay` 8.0)
  ;[1 1 1] 65
  (`GameplayStatics.PlaySound2D` "/Game/Sound/Seahorse/Audio_1_65.Audio_1_65" 1.0 1.0 0.0 null null)
  (`KismetSystemLibrary.Delay` 8.0)
  ;[1 1 1] 68
  (`GameplayStatics.PlaySound2D` "/Game/Sound/Seahorse/Audio_1_68.Audio_1_68" 1.0 1.0 0.0 null null)
  (`KismetSystemLibrary.Delay` 7.0)
  (`GameplayStatics.OpenLevelBySoftObjectPtr` "/Game/Levels/02_Library/Library_00.Library_00"))

(fn `UserConstructionScript`)