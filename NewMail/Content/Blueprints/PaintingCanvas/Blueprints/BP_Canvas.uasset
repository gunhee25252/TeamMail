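; BP_Canvas is a paintable surface that records brush hits in a render target driving the material on its Dust mesh.
; BeginPlay creates the render target, binds it to a dynamic masked translucent material on Dust, and creates a brush material instance.
; OnPaintVisualLineTrace converts a hit to UV, passes it with brush size, color and strength to that brush material, then draws it into the render target.
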(event `self.ReceiveBeginPlay`
  (bind _returnvalue (`PrimitiveComponent.CreateDynamicMaterialInstance` (`self.Dust`) 0 "/Game/Blueprints/PaintingCanvas/Materials/M_Masked_Trans_Inst.M_Masked_Trans_Inst" "None"))
  (bind _returnvalue_2 (`KismetRenderingLibrary.CreateRenderTarget2D` 1024 1024))
  (bind _output_get (set `self.RT` _returnvalue_2))
  (`MaterialInstanceDynamic.SetTextureParameterValue` _returnvalue "RT" _output_get)
  (bind _returnvalue_3 (`KismetMaterialLibrary.CreateDynamicMaterialInstance` "/Game/Blueprints/PaintingCanvas/Materials/MI_PaintBrush.MI_PaintBrush"))
  (set `self.BrushMaterialInstance` _returnvalue_3))

(fn `OnPaintVisualLineTrace`
  (params (PaintBrush :type "/Game/Blueprints/PaintingCanvas/Blueprints/BP_BlueCrayon Object Reference") (HitResult :type "HitResult Structure"))
  (bind (_x _y) (`KismetMathLibrary.BreakVector2D` (`GameplayStatics.FindCollisionUV` HitResult)))
  (set `self.Paint Brush` PaintBrush)
  (`MaterialInstanceDynamic.SetVectorParameterValue` (`self.BrushMaterialInstance`) "HitPosition" (make `LinearColor` _x _y 0.0 1.0))
  (`MaterialInstanceDynamic.SetScalarParameterValue` (`self.BrushMaterialInstance`) "BrushSize" (`/Game/Blueprints/PaintingCanvas/Blueprints/BP_BlueCrayon.BrushSize` (`self.Paint Brush`)))
  (`MaterialInstanceDynamic.SetVectorParameterValue` (`self.BrushMaterialInstance`) "BrushColor" (`KismetMathLibrary.Conv_ColorToLinearColor` (`/Game/Blueprints/PaintingCanvas/Blueprints/BP_BlueCrayon.BrushColor` (`self.Paint Brush`))))
  (`MaterialInstanceDynamic.SetScalarParameterValue` (`self.BrushMaterialInstance`) "BrushStrength" (`/Game/Blueprints/PaintingCanvas/Blueprints/BP_BlueCrayon.BrushStrength` (`self.Paint Brush`)))
  (`KismetRenderingLibrary.DrawMaterialToRenderTarget` (`self.RT`) (`self.BrushMaterialInstance`)))

(fn `UserConstructionScript`)