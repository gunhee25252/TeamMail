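; White crayon grabbable in the painting canvas content that starts a timed transition to the LoopBus_02 level.
; Its first grab sets the Paint flag, which also blocks repeat triggers.
; After a delay it activates the NSWindow effect on the referenced BPCanvas, then opens the level after a second delay.
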(event `self.GrabComponent.OnGrabbed`
  (if (not (`self.paint`))
    (set `self.paint` true)
    (`KismetSystemLibrary.Delay` 10.0)
    (`ActorComponent.Activate` (`/Game/Blueprints/PaintingCanvas/Blueprints/BP_Canvas.NS_Window` (`self.BP_Canvas`)) false)
    (`KismetSystemLibrary.Delay` 5.0)
    (`GameplayStatics.OpenLevelBySoftObjectPtr` "/Game/Levels/04_LoopBus/LoopBus_02.LoopBus_02")))

(fn `UserConstructionScript`
  (`parent.UserConstructionScript`))