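; Blue crayon actor that paints on a BP_Canvas while it is held.
; Each tick, if the GrabComponent reports it is held, it line-traces a short distance along its Arrow component.
; On a hit with a BP_Canvas, it passes itself as the paint brush, along with the hit result, to the canvas's OnPaintVisualLineTrace.
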(event `CheckInput`
  (bind _arrow (`self.Arrow`))
  (bind _returnvalue (`SceneComponent.K2_GetComponentLocation` _arrow))
  (if (`/Game/VRTemplate/Blueprints/GrabComponent.bIsHeld` (`self.GrabComponent`))
    (bind (_outhit _returnvalue_2) (`KismetSystemLibrary.LineTraceSingleByProfile` _returnvalue (+ _returnvalue (* (`SceneComponent.GetForwardVector` _arrow) 17.0)) "BlockAllDynamic" true))
    (if _returnvalue_2
      (bind _asbp_canvas (cast `/Game/Blueprints/PaintingCanvas/Blueprints/BP_Canvas` (`.HitActor` (`GameplayStatics.BreakHitResult` _outhit))))
      (`/Game/Blueprints/PaintingCanvas/Blueprints/BP_Canvas.OnPaintVisualLineTrace` _asbp_canvas self _outhit))))

(event `self.ReceiveTick`
  (params (DeltaSeconds :type "Float (single-precision)"))
  (`self.CheckInput`))

(fn `UserConstructionScript`)