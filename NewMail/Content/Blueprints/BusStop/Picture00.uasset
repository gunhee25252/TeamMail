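; Grabbable bus stop picture that, on its first grab only, triggers the 2D bus arrival sequence.
; A timeline animates the Strength of a dynamic material on the plane; after a short delay the plane hides and BusCard appears with its stencil call.
; Bus2D's Niagara activates and a second timeline slides the bus along X, while VRPawn's WB0002 and a stopping sound fire.
; The picture later destroys itself.
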(event `nnn`
  (bind _bus2d (`self.Bus2D`))
  (bind (_returnvalue_x _returnvalue_y) (`KismetMathLibrary.BreakVector` (`self.K2_GetActorLocation` _bus2d)))
  ;[1 1 1] Comment
  (`self.K2_SetActorLocation` _bus2d (`KismetMathLibrary.MakeVector` _returnvalue_x _returnvalue_y 34.145049) false false))

(event `self.GrabComponent.OnGrabbed`
  (bind _buscard (`self.BusCard`))
  (bind (_bus2dlocation_x _bus2dlocation_y _bus2dlocation_z) (`KismetMathLibrary.BreakVector` (`self.Bus2DLocation`)))
  (bind _bus2d (`self.Bus2D`))
  (if (not (`self.IsGrab`))
    (set `self.IsGrab` true)
    (bind _returnvalue (`PrimitiveComponent.CreateDynamicMaterialInstance` (`self.Plane`) 0 "/Game/Blueprints/BusStop/DefaultRibbonMaterial_NoGradient1.DefaultRibbonMaterial_NoGradient1" "None"))
    (bind _output_get (set `self.NewVar` _returnvalue))
    (`|ExecutionSequence`
      (:`then_0`
        (bind (_direction _newtrack_0) (`Timeline|Timeline_0`)
          (:`Update`
            (`MaterialInstanceDynamic.SetScalarParameterValue` _output_get "Strength" _newtrack_0))))
      (:`then_1`
        (`KismetSystemLibrary.Delay` 3.0)
        (`SceneComponent.SetHiddenInGame` (`self.Plane`) true false)
        (`self.SetActorHiddenInGame` _buscard false)
        (`/Game/Blueprints/Stencil_0/BusStation/BP_BusCard.BusCardStencil` _buscard)
        (`ActorComponent.Activate` (`/Game/Blueprints/Stencil_0/BusStation/BP_Bus_2D.Niagara` (`self.Bus2D`)) false)
        (bind _output_get_2 (set `self.Bus2DLocation` (`self.K2_GetActorLocation` _bus2d)))
        (`|ExecutionSequence`
          (:`then_0`
            (bind (_direction_2 _amount) (`Timeline|Timeline`)
              (:`Update`
                (`self.K2_SetActorLocation` _bus2d (`KismetMathLibrary.MakeVector` (+ (`KismetMathLibrary.Lerp` 0.0 (`self.BusMovement`) _amount) _bus2dlocation_x) _bus2dlocation_y _bus2dlocation_z) false false)
                (`KismetSystemLibrary.Delay` 10.0)
                (`self.K2_DestroyActor`))))
          (:`then_1`
            (bind _asvrpawn (cast `/Game/VRTemplate/Blueprints/VRPawn` (`GameplayStatics.GetPlayerPawn` 0)))
            (`/Game/VRTemplate/Blueprints/VRPawn.WB_0002` _asvrpawn)
            (`GameplayStatics.PlaySoundAtLocation` "/Game/Sound/BusStop/S_BusStopping.S_BusStopping" _output_get_2 (struct) 1.0 1.0 0.0 null null null null)))))))

(fn `UserConstructionScript`)