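; BP_End is the game's exit trigger in the last room, unlocked by ringing bells.
; Its RingBell event increments a counter and unhides a static mesh when the count reaches six.
; A box overlap by the VRPawn quits the game, but only while the count equals six.
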(event `self.Box.OnComponentBeginOverlap`
  (params (OverlappedComponent :type "PrimitiveComponent Object Reference") (OtherActor :type "Actor Object Reference") (OtherComp :type "PrimitiveComponent Object Reference") (OtherBodyIndex :type Integer) (bFromSweep :type Boolean) (SweepResult :type "HitResult Structure (by ref)"))
  (cast `/Game/VRTemplate/Blueprints/VRPawn` OtherActor)
  (if (== (`self.Count`) 6)
    (`KismetSystemLibrary.QuitGame` null "Quit")))

(event `RingBell`
  (set `self.Count` (+ (`self.Count`) 1))
  (if (== (`self.Count`) 6)
    (`SceneComponent.SetHiddenInGame` (`self.StaticMeshComponent`) false false)))

(fn `UserConstructionScript`)