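; BP_BusSignCube is a grabbable bus station cube that switches stencil highlighting across a set of bus sign pieces.
; Grabbing plays a pickup sound and shows the Effect actor, while dropping hides it.
; Both events call toggle functions on itself, the cone, sphere and bus sign.
; The cube's FlipFlop alternates its mesh's Custom Depth stencil value and Plane visibility, starting with stencil cleared and plane hidden.
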(event `self.GrabComponent.OnGrabbed`
  (`GameplayStatics.PlaySound2D` "/Game/LASTSound/BUS_STATION/BUS_STATION_GET.BUS_STATION_GET" 1.0 1.0 0.0 null null)
  (`self.CubeStencil`)
  (`/Game/Blueprints/Stencil_0/BusStation/BP_BusSignCone.ConeStencil` (`self.BusSignCone`))
  (`/Game/Blueprints/Stencil_0/BusStation/BP_BusSignSphere.SphereStencil` (`self.BusSignSphere`))
  (`/Game/Blueprints/Stencil_0/BusStation/BP_BusSign.BusSignStencil` (`self.BusSign`))
  (`self.SetActorHiddenInGame` (`self.Effect`) false))

(event `self.GrabComponent.OnDropped`
  (`self.CubeStencil`)
  (`/Game/Blueprints/Stencil_0/BusStation/BP_BusSignCone.ConeStencil` (`self.BusSignCone`))
  (`/Game/Blueprints/Stencil_0/BusStation/BP_BusSignSphere.SphereStencil` (`self.BusSignSphere`))
  (`/Game/Blueprints/Stencil_0/BusStation/BP_BusSign.BusSignStencil` (`self.BusSign`))
  (`self.SetActorHiddenInGame` (`self.Effect`) true))

(event `CubeStencil`
  (`/Engine/EditorBlueprintResources/StandardMacros.FlipFlop`
    (:`A`
      (`PrimitiveComponent.SetCustomDepthStencilValue` (`self.StaticMesh`) 0)
      (`SceneComponent.SetHiddenInGame` (`self.Plane`) true false))
    (:`B`
      (`PrimitiveComponent.SetCustomDepthStencilValue` (`self.StaticMesh`) 1)
      (`SceneComponent.SetHiddenInGame` (`self.Plane`) false false))))

(fn `UserConstructionScript`
  (`parent.UserConstructionScript`))