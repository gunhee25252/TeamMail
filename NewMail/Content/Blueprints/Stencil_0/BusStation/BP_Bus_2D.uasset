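; BP_Bus_2D is a bus at the bus station that acts as a card-activated transition into the InBus_03 level.
; When a BP_BusCard overlaps its Box, it plays card-tag and door-open sounds, then opens the level after a short delay.
; A separate BusStencil event uses a FlipFlop to toggle the bus's custom depth stencil value, unhiding StaticMesh on both branches.
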(event `self.Box.OnComponentBeginOverlap`
  (params (OverlappedComponent :type "PrimitiveComponent Object Reference") (OtherActor :type "Actor Object Reference") (OtherComp :type "PrimitiveComponent Object Reference") (OtherBodyIndex :type Integer) (bFromSweep :type Boolean) (SweepResult :type "HitResult Structure (by ref)"))
  (cast `/Game/Blueprints/Stencil_0/BusStation/BP_BusCard` OtherActor)
  (`GameplayStatics.PlaySoundAtLocation` "/Game/LASTSound/BUS_STATION/BUS_STATION_CARD_TAG.BUS_STATION_CARD_TAG" (`SceneComponent.K2_GetComponentLocation` (`self.Box`)) (struct) 1.0 1.0 0.0 null null null null)
  (`GameplayStatics.PlaySound2D` "/Game/LASTSound/BUS_STATION/BUS_STATION_DOOR_OPEN.BUS_STATION_DOOR_OPEN" 1.0 1.0 0.0 null null)
  (`KismetSystemLibrary.Delay` 1.0)
  (`GameplayStatics.OpenLevelBySoftObjectPtr` "/Game/Levels/03_InBus/InBus_03.InBus_03"))

(event `BusStencil`
  (bind _staticmesh (`self.StaticMesh`))
  (bind _bus_2d_v02 (`self.bus_2d_v02`))
  (`/Engine/EditorBlueprintResources/StandardMacros.FlipFlop`
    (:`A`
      (`PrimitiveComponent.SetCustomDepthStencilValue` _bus_2d_v02 1)
      (`SceneComponent.SetHiddenInGame` _staticmesh false false))
    (:`B`
      (`PrimitiveComponent.SetCustomDepthStencilValue` _bus_2d_v02 0)
      (`SceneComponent.SetHiddenInGame` _staticmesh false false))))

(fn `UserConstructionScript`)