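; BP_BusCard is a grabbable bus card in the bus station that changes custom depth stencil values as it is picked up and dropped.
; Grabbing plays a pickup sound, and both grab and drop fire the card's stencil toggle and call BusStencil on Bus2D.
; The card's toggle uses a FlipFlop to alternate its mesh stencil between on and off, so it relies on call order rather than held state.
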(event `self.GrabComponent.OnGrabbed`
  (`GameplayStatics.PlaySound2D` "/Game/LASTSound/BUS_STATION/BUS_STATION_BUSSIGN_CARD_GET.BUS_STATION_BUSSIGN_CARD_GET" 1.0 1.0 0.0 null null)
  (`self.BusCardStencil`)
  (`/Game/Blueprints/Stencil_0/BusStation/BP_Bus_2D.BusStencil` (`self.Bus2D`)))

(event `self.GrabComponent.OnDropped`
  (`self.BusCardStencil`)
  (`/Game/Blueprints/Stencil_0/BusStation/BP_Bus_2D.BusStencil` (`self.Bus2D`)))

(event `BusCardStencil`
  (`/Engine/EditorBlueprintResources/StandardMacros.FlipFlop`
    (:`A`
      (`PrimitiveComponent.SetCustomDepthStencilValue` (`self.StaticMesh`) 1))
    (:`B`
      (`PrimitiveComponent.SetCustomDepthStencilValue` (`self.StaticMesh`) 0))))

(fn `UserConstructionScript`
  (`parent.UserConstructionScript`))