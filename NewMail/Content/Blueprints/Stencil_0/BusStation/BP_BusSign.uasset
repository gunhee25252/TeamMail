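; Bus sign puzzle actor for a VR scene that collects cone, cube and sphere pieces to produce the bus card.
; Each piece overlapping the Box is destroyed, toggles custom-depth stencils on the signs, spawns a card shape and plays a ping.
; With all three collected, it notifies the VRPawn and swaps the 2D bus stop for 3D.
; After a delay, it reveals the card and places a picture before the player.
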(event `self.Box.OnComponentBeginOverlap`
  (params (OverlappedComponent :type "PrimitiveComponent Object Reference") (OtherActor :type "Actor Object Reference") (OtherComp :type "PrimitiveComponent Object Reference") (OtherBodyIndex :type Integer) (bFromSweep :type Boolean) (SweepResult :type "HitResult Structure (by ref)"))
  (bind _returnvalue (`GameplayStatics.GetPlayerPawn` 0))
  (bind _returnvalue_2 (`SceneComponent.K2_GetComponentLocation` (`self.Box`)))
  (bind _returnvalue_3 (`SceneComponent.K2_GetComponentLocation` (`self.Box`)))
  (bind _returnvalue_4 (`SceneComponent.K2_GetComponentLocation` (`self.Box`)))
  (if (not (`self.IsThereBuscard`))
    (`|ExecutionSequence`
      (:`then_0`
        (bind _asbp_bus_sign_cone (cast `/Game/Blueprints/Stencil_0/BusStation/BP_BusSignCone` OtherActor))
        (set `self.IsThereCone` true)
        (`self.K2_DestroyActor` _asbp_bus_sign_cone)
        (`self.BusSignStencil`)
        (`/Game/Blueprints/Stencil_0/BusStation/BP_BusSignCone.ConeStencil` (`self.SignCone`))
        (`/Game/Blueprints/Stencil_0/BusStation/BP_BusSignCube.CubeStencil` (`self.SignCube`))
        (`/Game/Blueprints/Stencil_0/BusStation/BP_BusSignSphere.SphereStencil` (`self.SignSphere`))
        (bind _returnvalue_5 (`|SpawnActorFromClass` "/Game/Blueprints/BusCard/CardCone.CardCone_C" (`KismetMathLibrary.MakeTransform` (+ _returnvalue_2 (-10.0 10.781838 0.0)) (struct) (0.5 0.5 0.5)) "AlwaysSpawn" "MultiplyWithRoot" null null))
        (`GameplayStatics.PlaySoundAtLocation` "/Engine/EngineSounds/1kSineTonePing.1kSineTonePing" _returnvalue_2 (struct) 1.0 1.0 0.0 null null null null)
        (`self.SetActorHiddenInGame` (`self.Effect`) true :!label _label))
      (:`then_1`
        (bind _asbp_bus_sign_cube (cast `/Game/Blueprints/Stencil_0/BusStation/BP_BusSignCube` OtherActor))
        (set `self.IsThereCube` true)
        (`self.K2_DestroyActor` _asbp_bus_sign_cube)
        (`self.BusSignStencil`)
        (`/Game/Blueprints/Stencil_0/BusStation/BP_BusSignCone.ConeStencil` (`self.SignCone`))
        (`/Game/Blueprints/Stencil_0/BusStation/BP_BusSignCube.CubeStencil` (`self.SignCube`))
        (`/Game/Blueprints/Stencil_0/BusStation/BP_BusSignSphere.SphereStencil` (`self.SignSphere`))
        (bind _returnvalue_6 (`|SpawnActorFromClass` "/Game/Blueprints/BusCard/CardCube.CardCube_C" (`KismetMathLibrary.MakeTransform` (+ _returnvalue_4 (-10.0 0.0 0.0)) (struct) (0.5 0.5 0.5)) "AlwaysSpawn" "MultiplyWithRoot" null null))
        (`GameplayStatics.PlaySoundAtLocation` "/Engine/EngineSounds/1kSineTonePing.1kSineTonePing" _returnvalue_4 (struct) 1.0 1.0 0.0 null null null null)
        (goto _label))
      (:`then_2`
        (bind _asbp_bus_sign_sphere (cast `/Game/Blueprints/Stencil_0/BusStation/BP_BusSignSphere` OtherActor))
        (set `self.IsThereSphere` true)
        (`self.K2_DestroyActor` _asbp_bus_sign_sphere)
        (`self.BusSignStencil`)
        (`/Game/Blueprints/Stencil_0/BusStation/BP_BusSignCone.ConeStencil` (`self.SignCone`))
        (`/Game/Blueprints/Stencil_0/BusStation/BP_BusSignCube.CubeStencil` (`self.SignCube`))
        (`/Game/Blueprints/Stencil_0/BusStation/BP_BusSignSphere.SphereStencil` (`self.SignSphere`))
        (bind _returnvalue_7 (`|SpawnActorFromClass` "/Game/Blueprints/BusCard/CardSphere.CardSphere_C" (`KismetMathLibrary.MakeTransform` (+ _returnvalue_3 (-10.0 -13.7303 0.0)) (struct) (0.5 0.5 0.5)) "AlwaysSpawn" "MultiplyWithRoot" null null))
        (`GameplayStatics.PlaySoundAtLocation` "/Engine/EngineSounds/1kSineTonePing.1kSineTonePing" _returnvalue_3 (struct) 1.0 1.0 0.0 null null null null)
        (goto _label))
      (:`then_3`
        (if (and (`self.IsThereCone`) (`self.IsThereCube`) (`self.IsThereSphere`))
          (set `self.IsThereBuscard` true)
          (bind _asvrpawn (cast `/Game/VRTemplate/Blueprints/VRPawn` (`GameplayStatics.GetPlayerPawn` 0)))
          (`/Game/VRTemplate/Blueprints/VRPawn.WB_002` _asvrpawn)
          (`SceneComponent.SetHiddenInGame` (`self.SkeletalMesh`) true false)
          (`/Game/Blueprints/Stencil_0/BusStation/BP_BusStop2D.BusStop2DIsDisappear` (`self.BusStop2D`))
          (`/Game/VFX/BusStop2/BP_disin.BusStop3DIsAppear` (`self.BusStop3D`))
          (`self.K2_DestroyActor` (`self.BusCardBefore`))
          (`self.K2_DestroyActor` _returnvalue_5)
          (`self.K2_DestroyActor` _returnvalue_6)
          (`self.K2_DestroyActor` _returnvalue_7)
          (`KismetSystemLibrary.Delay` 5.0)
          (`SceneComponent.SetHiddenInGame` (`self.StaticMesh`) false false)
          (`SceneComponent.SetHiddenInGame` (`Actor.RootComponent` (`self.BusCard`)) false false)
          (bind _asvrpawn_2 (cast `/Game/VRTemplate/Blueprints/VRPawn` _returnvalue))
          (`SceneComponent.K2_SetWorldLocationAndRotation` (`Actor.RootComponent` (`self.Picture00`)) (+ (`SceneComponent.K2_GetComponentLocation` (`Actor.RootComponent` _returnvalue)) (* (`self.GetActorForwardVector` _returnvalue) 50)) (`SceneComponent.K2_GetComponentRotation` (`/Game/VRTemplate/Blueprints/VRPawn.Camera` _asvrpawn_2)) false false))))))

(event `BusSignStencil`
  (bind _skeletalmesh (`self.SkeletalMesh`))
  (`/Engine/EditorBlueprintResources/StandardMacros.FlipFlop`
    (:`A`
      (`PrimitiveComponent.SetCustomDepthStencilValue` _skeletalmesh 1))
    (:`B`
      (`PrimitiveComponent.SetCustomDepthStencilValue` _skeletalmesh 0))))

(fn `UserConstructionScript`
  (`parent.UserConstructionScript`))